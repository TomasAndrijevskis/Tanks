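; BP_TanksGameMode is the game mode for a tanks game, handling pause and unpause.
; On BeginPlay it stores the current level name.
; Its PauseGame event sets the game's paused state, then either creates a WBP_Pause widget for the first player and adds it to the viewport, or removes the stored widget when unpausing.
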(event Custom|PauseGame
  (params (IsPaused :type Boolean))
  (Game|SetGamePaused IsPaused)
  (if IsPaused
    (bind _returnvalue (UserInterface|CreateWidget "/Game/Widgets/WBP_Pause.WBP_Pause_C" (Game|GetPlayerController 0)))
    (bind _output_get (Variables|Default|SetRef_PauseScreen _returnvalue))
    (UserInterface|Viewport|AddtoViewport _output_get 0)
    (else
      (Widget|RemovefromParent (Variables|Default|GetRef_PauseScreen)))))

(event EventBeginPlay
  (bind _returnvalue (Game|GetCurrentLevelName true))
  (Variables|Default|SetCurrentLevelName _returnvalue))

(fn ConstructionScript)